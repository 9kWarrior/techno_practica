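; Game state that runs an endless Bot0 arena and tallies which randomized bot builds survive.
; When fewer than two bots exist, Tick spawns one with random stats, resets the survivor's lifetime and records its win.
; WinTotalArray keys concatenate stats and fight results, though lookups use only the first four characters.
; EndPlay saves the tallies to a text file; BeginPlay only prints a differently named file.
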(event Custom|PrintAllWins
  (bind _wintotalarray (Variables|Default|GetWinTotalArray))
  (bind _keys (Utilities|Map|Keys _wintotalarray))
  (for _array_element _keys
    (if (.ReturnValue (Utilities|Map|Find _wintotalarray _array_element))
      (Development|PrintString (Utilities|String|Append _array_element " " (Utilities|String|ToString(Integer) (.Value (Utilities|Map|Find _wintotalarray _array_element))) " ")))))

(event Custom|SaveToFileAsTxt
  (Variables|Default|SetstringOfbotWins "")
  (bind _keys (Utilities|Map|Keys (Variables|Default|GetWinTotalArray)))
  (for _array_element _keys
    (Variables|Default|SetstringOfbotWins (Utilities|String|Append (Variables|Default|GetstringOfbotWins) (Utilities|String|Append _array_element " " (Utilities|String|ToString(Integer) (.Value (Utilities|Map|Find (Variables|Default|GetWinTotalArray) _array_element))) " "))))
  (Class|RWTxtFile|SaveTxt (Utilities|String|Append (Variables|Default|Getteststring) (Variables|Default|GetstringOfbotWins)) "botwins2.txt"))

(event EventBeginPlay
  (Development|PrintString (.SaveTextA (Class|RWTxtFile|LoadTxt "botwins4,txt"))))

(event EventTick
  (params (DeltaSeconds :type Float%20%28single-precision%29))
  (bind _returnvalue (Math|Random|RandomIntegerinRange 330 2500))
  (bind _returnvalue_2 (Math|Random|RandomIntegerinRange 330 2500))
  (bind _wintotalarray (Variables|Default|GetWinTotalArray))
  (bind _returnvalue_3 (Math|Conversions|ToFloat(Integer) _returnvalue_2))
  (bind _returnvalue_4 (Math|Conversions|ToFloat(Integer) _returnvalue))
  (bind _outactors (Actor|GetAllActorsOfClass "/Game/AI/Bot0.Bot0_C"))
  (if (< (Utilities|Array|Length _outactors) 2)
    (bind _returnvalue_5 (Game|SpawnActorfromClass "/Game/AI/Bot0.Bot0_C" (Math|Transform|MakeTransform (Math|Vector|MakeVector _returnvalue_3 _returnvalue_4 5e+02) "0, 0, 0" "0.500000,0.500000,0.500000") "Undefined" "MultiplyWithRoot" 0 0))
    (Variables|/Game/AI/Bot0.Bot0_C|SetBasicPunchLvl _returnvalue_5 (Math|Random|RandomIntegerinRange 1 4))
    (Variables|/Game/AI/Bot0.Bot0_C|SetSpeedMultip _returnvalue_5 (Math|Conversions|ToFloat(Integer) (Math|Random|RandomIntegerinRange 1 3000)))
    (Variables|/Game/AI/Bot0.Bot0_C|SetTurnRatio _returnvalue_5 (Math|Random|RandomIntegerinRange 1 9))
    (Variables|/Game/AI/Bot0.Bot0_C|SetSpawnLocationX _returnvalue_5 (Utilities|String|ToString(Integer) (Class|KismetMathLibrary|ToInt64(Float) _returnvalue_3)))
    (Variables|/Game/AI/Bot0.Bot0_C|SetSpawnLocationY _returnvalue_5 (Utilities|String|ToString(Integer) (Class|KismetMathLibrary|ToInt64(Float) _returnvalue_4)))
    (Variables|/Game/AI/Bot0.Bot0_C|SetMassOfBot _returnvalue_5 (Math|Conversions|ToFloat(Integer) (* (Math|Random|RandomIntegerinRange 1 5) 600)))
    (for _array_element _outactors
      (Variables|/Game/AI/Bot0.Bot0_C|SetLifetime _array_element 1e+01)
      (if (.ReturnValue (Utilities|Map|Find _wintotalarray (Utilities|String|Left (Utilities|String|Append (Utilities|String|Right (Utilities|String|Append "000" (Utilities|String|ToString(Integer) (Math|Float|Truncate (Variables|/Game/AI/Bot0.Bot0_C|GetSpeedMultip _array_element)))) 4) " " (Utilities|String|ToString(Integer) (Variables|/Game/AI/Bot0.Bot0_C|GetTurnRatio _array_element)) " " (Utilities|String|ToString(Integer) (Class|KismetMathLibrary|FTrunc64 (Variables|/Game/AI/Bot0.Bot0_C|GetSurviveTime _array_element))) " " (Utilities|String|ToString(Integer) (Variables|/Game/AI/Bot0.Bot0_C|GetDonePunchs _array_element)) " " (Utilities|String|ToString(Integer) (Math|Conversions|ToInteger(Boolean) (Variables|Default|GetDeadByTimer))) " " (Utilities|String|ToString(Integer) (Variables|/Game/AI/Bot0.Bot0_C|GetBasicPunchLvl _array_element)) " " (Variables|/Game/AI/Bot0.Bot0_C|GetSpawnLocationX _array_element) " " (Variables|/Game/AI/Bot0.Bot0_C|GetSpawnLocationY _array_element) " " (Utilities|String|ToString(Integer) (Class|KismetMathLibrary|ToInt64(Float) (Variables|/Game/AI/Bot0.Bot0_C|GetMassOfBot _array_element)))) 4)))
        (Utilities|Map|Add _wintotalarray (Utilities|String|Append (Utilities|String|Right (Utilities|String|Append "000" (Utilities|String|ToString(Integer) (Math|Float|Truncate (Variables|/Game/AI/Bot0.Bot0_C|GetSpeedMultip _array_element)))) 4) " " (Utilities|String|ToString(Integer) (Variables|/Game/AI/Bot0.Bot0_C|GetTurnRatio _array_element)) " " (Utilities|String|ToString(Integer) (Class|KismetMathLibrary|FTrunc64 (Variables|/Game/AI/Bot0.Bot0_C|GetSurviveTime _array_element))) " " (Utilities|String|ToString(Integer) (Variables|/Game/AI/Bot0.Bot0_C|GetDonePunchs _array_element)) " " (Utilities|String|ToString(Integer) (Math|Conversions|ToInteger(Boolean) (Variables|Default|GetDeadByTimer))) " " (Utilities|String|ToString(Integer) (Variables|/Game/AI/Bot0.Bot0_C|GetBasicPunchLvl _array_element)) " " (Variables|/Game/AI/Bot0.Bot0_C|GetSpawnLocationX _array_element) " " (Variables|/Game/AI/Bot0.Bot0_C|GetSpawnLocationY _array_element) " " (Utilities|String|ToString(Integer) (Class|KismetMathLibrary|ToInt64(Float) (Variables|/Game/AI/Bot0.Bot0_C|GetMassOfBot _array_element)))) (+ (.Value (Utilities|Map|Find _wintotalarray (Utilities|String|Left (Utilities|String|Append (Utilities|String|Right (Utilities|String|Append "000" (Utilities|String|ToString(Integer) (Math|Float|Truncate (Variables|/Game/AI/Bot0.Bot0_C|GetSpeedMultip _array_element)))) 4) " " (Utilities|String|ToString(Integer) (Variables|/Game/AI/Bot0.Bot0_C|GetTurnRatio _array_element)) " " (Utilities|String|ToString(Integer) (Class|KismetMathLibrary|FTrunc64 (Variables|/Game/AI/Bot0.Bot0_C|GetSurviveTime _array_element))) " " (Utilities|String|ToString(Integer) (Variables|/Game/AI/Bot0.Bot0_C|GetDonePunchs _array_element)) " " (Utilities|String|ToString(Integer) (Math|Conversions|ToInteger(Boolean) (Variables|Default|GetDeadByTimer))) " " (Utilities|String|ToString(Integer) (Variables|/Game/AI/Bot0.Bot0_C|GetBasicPunchLvl _array_element)) " " (Variables|/Game/AI/Bot0.Bot0_C|GetSpawnLocationX _array_element) " " (Variables|/Game/AI/Bot0.Bot0_C|GetSpawnLocationY _array_element) " " (Utilities|String|ToString(Integer) (Class|KismetMathLibrary|ToInt64(Float) (Variables|/Game/AI/Bot0.Bot0_C|GetMassOfBot _array_element)))) 4))) 1))
        (Variables|Default|SetDeadByTimer false)
        (else
          (Utilities|Map|Add _wintotalarray (Utilities|String|Append (Utilities|String|Right (Utilities|String|Append "000" (Utilities|String|ToString(Integer) (Math|Float|Truncate (Variables|/Game/AI/Bot0.Bot0_C|GetSpeedMultip _array_element)))) 4) " " (Utilities|String|ToString(Integer) (Variables|/Game/AI/Bot0.Bot0_C|GetTurnRatio _array_element)) " " (Utilities|String|ToString(Integer) (Class|KismetMathLibrary|FTrunc64 (Variables|/Game/AI/Bot0.Bot0_C|GetSurviveTime _array_element))) " " (Utilities|String|ToString(Integer) (Variables|/Game/AI/Bot0.Bot0_C|GetDonePunchs _array_element)) " " (Utilities|String|ToString(Integer) (Math|Conversions|ToInteger(Boolean) (Variables|Default|GetDeadByTimer))) " " (Utilities|String|ToString(Integer) (Variables|/Game/AI/Bot0.Bot0_C|GetBasicPunchLvl _array_element)) " " (Variables|/Game/AI/Bot0.Bot0_C|GetSpawnLocationX _array_element) " " (Variables|/Game/AI/Bot0.Bot0_C|GetSpawnLocationY _array_element) " " (Utilities|String|ToString(Integer) (Class|KismetMathLibrary|ToInt64(Float) (Variables|/Game/AI/Bot0.Bot0_C|GetMassOfBot _array_element)))) 1)
          (Variables|Default|SetDeadByTimer false))))))

(event EventEndPlay
  (params (EndPlayReason :type EEndPlayReason%20Enum :default "Destroyed"))
  (CallFunction|SavetoFileasTxt))

(fn ConstructionScript)